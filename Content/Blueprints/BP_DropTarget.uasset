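; BP_DropTarget is a pinball drop target that sinks when hit and displays a letter set at construction.
; On Hit it drops, playing a sound, moving its mesh down and disabling collision, then fires the OnDrop dispatcher.
; ResetTarget moves the mesh back and restores collision.
; At BeginPlay it binds an event to the pinball game mode's OnGameReset dispatcher.
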(event Custom|Drop
  (bind _dtmesh (Variables|Default|GetDTMesh))
  (Audio|PlaySoundatLocation "/Game/Sound/DropTargetOnDrop.DropTargetOnDrop" (Transformation|GetActorLocation))
  (Components|MoveComponentTo _dtmesh "0, 0,-110.000000" "0, 0, 0" false false 0.2 false)
  (Collision|SetCollisionEnabled _dtmesh "NoCollision"))

(event Custom|ResetTarget
  (bind _dtmesh (Variables|Default|GetDTMesh))
  (Components|MoveComponentTo _dtmesh "0, 0, 0" "0, 0, 0" false false 0.2 false)
  (Collision|SetCollisionEnabled _dtmesh "QueryAndPhysics"))

(event EventBeginPlay
  (bind _asgm_pin_ball (Utilities|Casting|CastToGM_PinBall (Game|GetGameMode)))
  (EventDispatchers|BindEventtoOnGameReset _asgm_pin_ball (EventDispatchers|CreateEvent :!event Custom|ResetTarget)))

(event Collision|EventActorBeginOverlap
  (params (OtherActor :type Actor%20Object%20Reference)))

(event EventTick
  (params (DeltaSeconds :type Float%20%28single-precision%29)))

(event Collision|EventHit
  (params (MyComp :type Primitive%20Component%20Object%20Reference) (Other :type Actor%20Object%20Reference) (OtherComp :type Primitive%20Component%20Object%20Reference) (bSelfMoved :type Boolean) (HitLocation :type Vector :default "0, 0, 0") (HitNormal :type Vector :default "0, 0, 0") (NormalImpulse :type Vector :default "0, 0, 0") (Hit :type Hit%20Result%20Structure%20%28by%20ref%29))
  (CallFunction|Drop)
  (Default|CallOnDrop))

(fn ConstructionScript
  (Rendering|Components|TextRender|SetText (Variables|Default|GetTextRender) (Utilities|Text|ToText(String) (Variables|Default|GetDropLetter))))