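; SG_HighScore is a high-score object, likely a SaveGame, that holds score entries in the SaveStruct array.
; AddHighScore appends a new entry, sorts the array, then trims it to at most the requested length.
; SortSaveData orders scores from highest to lowest with a selection sort, repeatedly moving DetermineHighestVal's result into a temporary array.
; DetermineLowestVal returns the lowest entry and index but is not called here.
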(fn DetermineLowestVal
  (bind _savestruct (Variables|Default|GetSaveStruct))
  (for (_array_element _array_index) _savestruct
    (if (== _array_index 0)
      (LocalVariables|SetLowestScore (.score _array_element))
      (LocalVariables|SetLowestIndex _array_index)
      (elif (< (.score _array_element) (LocalVariables|GetLowestScore))
        (LocalVariables|SetLowestScore (.score _array_element))
        (LocalVariables|SetLowestIndex _array_index))))
  (return (Utilities|Array|Get(acopy) _savestruct (LocalVariables|GetLowestIndex)) (LocalVariables|GetLowestIndex)))

(fn DetermineHighestVal
  (bind _savestruct (Variables|Default|GetSaveStruct))
  (for (_array_element _array_index) _savestruct
    (if (== _array_index 0)
      (LocalVariables|SetHighestScore (.score _array_element))
      (LocalVariables|SetHighestIndex _array_index)
      (elif (> (.score _array_element) (LocalVariables|GetHighestScore))
        (LocalVariables|SetHighestScore (.score _array_element))
        (LocalVariables|SetHighestIndex _array_index))))
  (return (Utilities|Array|Get(acopy) _savestruct (LocalVariables|GetHighestIndex)) (LocalVariables|GetHighestIndex)))

(fn SortSaveData
  (while (> (Utilities|Array|Length (Variables|Default|GetSaveStruct)) 0)
    (bind (_highestscorestruct _highestscoreindex) (CallFunction|DetermineHighestVal))
    (Utilities|Array|Add (LocalVariables|GetTmpSaveStruct) _highestscorestruct)
    (Utilities|Array|RemoveIndex (Variables|Default|GetSaveStruct) _highestscoreindex))
  (Variables|Default|SetSaveStruct (LocalVariables|GetTmpSaveStruct)))

(fn AddHighScore
  (params (NewScoreStruct :type ST%20High%20Score%20Structure) (HighScoreLength :type Integer))
  (bind _savestruct (Variables|Default|GetSaveStruct))
  (Utilities|Array|Add _savestruct NewScoreStruct)
  (CallFunction|SortSaveData)
  (Utilities|Array|Resize _savestruct (Math|Integer|Min(Integer) HighScoreLength (Utilities|Array|Length _savestruct))))