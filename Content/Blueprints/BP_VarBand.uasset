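; BP_VarBand is a construction-script-only actor that builds a variable-length band between two posts.
; Post1 and a spawned Post2, which copies its mesh and sits at PostLocation, are rotated to face each other.
; A second added mesh component starts at Post1's transform and stretches along X by the post distance divided by 100, keeping Post1's Y and Z scale.
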(event EventBeginPlay)

(event Collision|EventActorBeginOverlap
  (params (OtherActor :type Actor%20Object%20Reference)))

(event EventTick
  (params (DeltaSeconds :type Float%20%28single-precision%29)))

(fn ConstructionScript
  (bind _post1 (Variables|Default|GetPost1))
  (bind _postlocation (Variables|Default|GetPostLocation))
  (bind _returnvalue (Transformation|GetRelativeTransform _post1))
  (bind _relativelocation (Variables|/Script/Engine.SceneComponent|GetRelativeLocation _post1))
  (bind (_location _rotation _scale) (Math|Transform|BreakTransform _returnvalue))
  (Transformation|SetRelativeRotation _post1 (Math|Rotator|FindLookatRotation _relativelocation _postlocation) false false)
  (bind _returnvalue_2 (AddComponent|AddStaticMeshComponent false (Math|Transform|MakeTransform _postlocation (Math|Rotator|FindLookatRotation _postlocation _relativelocation))))
  (bind _output_get (Variables|Default|SetPost2 _returnvalue_2))
  (Components|StaticMesh|SetStaticMesh _output_get (Variables|/Script/Engine.StaticMeshComponent|GetStaticMesh _post1))
  (bind _returnvalue_3 (AddComponent|AddStaticMeshComponent false _returnvalue))
  (Transformation|SetRelativeScale3D _returnvalue_3 (Math|Vector|MakeVector (/ (Math|Vector|VectorLength (- _location (Variables|Default|GetPostLocation))) 1e+02) (.y _scale) (.z _scale))))