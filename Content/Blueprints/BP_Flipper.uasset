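; BP_Flipper is a left or right flipper actor that swings between a rest and a flipped rotation.
; The construction script derives mirrored start and end rotations from FlipType, applies the start pose, and negates X scale for the right side so one component serves both sides.
; Flip and Flop events tween the Flipper component to the end or start rotation over FlipTime using MoveComponentTo.
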(event Custom|Flip
  (Components|MoveComponentTo (Variables|Default|GetFlipper) "0, 0, 0" (Variables|Default|GetEndRot) false false (Variables|Default|GetFlipTime) false))

(event Custom|Flop
  (Components|MoveComponentTo (Variables|Default|GetFlipper) "0, 0, 0" (Variables|Default|GetStartRot) false false (Variables|Default|GetFlipTime) false))

(event EventBeginPlay)

(event Collision|EventActorBeginOverlap
  (params (OtherActor :type Actor%20Object%20Reference)))

(event EventTick
  (params (DeltaSeconds :type Float%20%28single-precision%29)))

(fn ConstructionScript
  (bind _fliptype (Variables|Default|GetFlipType))
  (bind _flipper (Variables|Default|GetFlipper))
  (bind _returnvalue (Utilities|Select :Index _fliptype :NewEnumerator0 "0,20.000000, 0" :NewEnumerator1 "0,-20.000000, 0"))
  (bind _output_get (Variables|Default|SetStartRot _returnvalue))
  (Variables|Default|SetEndRot (* _returnvalue -1.0))
  (Transformation|SetRelativeRotation _flipper _output_get false false)
  (switch Utilities|FlowControl|Switch|SwitchonFlipType _fliptype
    (:NewEnumerator1
      (Transformation|SetRelativeScale3D _flipper "-1.000000,1.000000,1.000000"))))